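; Touch component for the AR Furniture app that detects one-finger swipe gestures and reports them to a GestureManager.
; A press records the start position and opens a timed window, closed by a delay of SwipeTime.
; A release inside that window and beyond MinSwipeDistance fires a generic swipe with its vector, plus a left, right, up or down call chosen by the dominant axis.
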(event Custom|Finger1_Pressed
  (params (TouchPosition :type Vector%202D%20Structure))
  (Variables|Default|SetStartTouchPosition TouchPosition)
  (Variables|Default|SetIsSwipe true)
  (Utilities|FlowControl|Delay (Variables|Default|GetSwipeTime))
  (Variables|Default|SetIsSwipe false))

(event Custom|Finger1_Released
  (params (TouchPosition :type Vector%202D%20Structure))
  (bind _gesturemanager (Variables|Default|GetGestureManager))
  (bind _starttouchposition (Variables|Default|GetStartTouchPosition))
  (bind _gesturemanager_2 (Variables|Default|GetGestureManager))
  (bind _returnvalue (- TouchPosition _starttouchposition))
  (bind (_x _y) (Math|Vector2D|BreakVector2D _returnvalue))
  (if (Variables|Default|GetIsSwipe)
    (if (> (Math|Vector2D|Vector2DLength _returnvalue) (Variables|Default|GetMinSwipeDistance))
      (Variables|Default|SetIsSwipe false)
      (Default|CallonSwipe (Variables|Default|GetGestureManager) _returnvalue)
      ;[1 1 1] Check if horizontal or vertical
      (if (> (Math|Float|Absolute(Float) _x) (Math|Float|Absolute(Float) _y))
        (if (> _x 0.0)
          (Default|CallonSwipeRight _gesturemanager)
          (else
            (Default|CallonSwipeLeft _gesturemanager)))
        (elif (> _y 0.0)
          (Default|CallonSwipeDown _gesturemanager_2)
          (else
            (Default|CallonSwipeUp _gesturemanager_2))))
      (else
        (Development|PrintString "Swipe is too short")))
    (else
      (Development|PrintString "Swipe is too long in time"))))