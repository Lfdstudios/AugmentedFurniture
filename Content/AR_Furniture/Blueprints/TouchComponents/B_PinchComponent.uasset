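; Touch component that detects two-finger pinch gestures in the AR furniture app.
; StartPitch records the initial distance between the fingers, and UpdatePitch measures the change from the stored distance.
; Changes above PinchThreshold update that distance and pass the signed delta to GestureManager's CallOnPitch, except large jumps, which are absorbed without being reported.
; Changes under the threshold leave the stored distance untouched, so slow pinches accumulate until they register.
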(event Custom|StartPitch
  (params (Finger1_TouchPos :type Vector%202D%20Structure) (Finger2_TouchPos :type Vector%202D%20Structure))
  (Variables|Default|SetPreviousPinchValue (Math|Vector2D|Vector2DLength (- Finger1_TouchPos Finger2_TouchPos)))
  (Development|PrintString "Start Pitch"))

(event Custom|UpdatePitch
  (params (Finger1_TouchPos :type Vector%202D%20Structure) (Finger2_TouchPos :type Vector%202D%20Structure))
  (bind _returnvalue (- Finger1_TouchPos Finger2_TouchPos))
  (bind _returnvalue_2 (Math|Vector2D|Vector2DLength _returnvalue))
  (if (> (Math|Float|Absolute(Float) (- _returnvalue_2 (Variables|Default|GetPreviousPinchValue))) (Variables|Default|GetPinchThreshold))
    (if (< (Math|Float|Absolute(Float) (- _returnvalue_2 (Variables|Default|GetPreviousPinchValue))) 1e+02)
      (Default|CallonPitch (Variables|Default|GetGestureManager) (- _returnvalue_2 (Variables|Default|GetPreviousPinchValue))))
    (Variables|Default|SetPreviousPinchValue _returnvalue_2)))