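; Touch gesture manager for the AR furniture project, turning finger input into tap, double tap, drag, swipe, pinch and rotate events.
; It registers itself with five gesture components and feeds them touch positions, using timelines for one- and two-finger updates.
; Components call back into the manager, which relays gestures, gating pinch and rotate on a PinchRotate switch.
; A double tap briefly raises a flag meant to prevent spawning.
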(event Custom|CallOnDoubleTap
  ;[1 1 1] Tap Component Events
  (Default|CallOnDoubleTap)
  (Development|PrintString "Double Tap")
  ;[1 1 1] For not spawn after double tap
  (Variables|Default|SetDoubleTap true)
  (Utilities|FlowControl|Delay 0.2)
  (Variables|Default|SetDoubleTap false))

(event Custom|CallOnPitch
  (params (PinchDelta :type Float%20%28single-precision%29))
  ;[0 0.3278 0] Pitch Component Events
  (switch Utilities|FlowControl|Switch|SwitchonEnumPinchRotate (Variables|Default|GetPinchRotate)
    (:NewEnumerator0
      (Default|CallOnPinch PinchDelta) ; For zoom 2 fingers
    )))

(event Custom|CallOnSwipeUp
  ;[1 1 1] Swipe Component Events
  (Default|CallOnSwipeUp)
  (Development|PrintString "Swipe UP"))

(event Custom|CallOnSwipeDown
  ;[1 1 1] Swipe Component Events
  (Default|CallOnSwipeDown)
  (Development|PrintString "Swipe DOWN"))

(event Custom|CallOnSwipeLeft
  ;[1 1 1] Swipe Component Events
  (Default|CallOnSwipeLeft)
  (Development|PrintString "Swipe LEFT"))

(event Custom|CallOnSwipeRight
  ;[1 1 1] Swipe Component Events
  (Default|CallOnSwipeRight)
  (Development|PrintString "Swipe RIGHT"))

(event Custom|CallOnDrag
  (params (DragDelta :type Vector%202D%20Structure))
  ;[1 1 1] Drag Component Events
  (Default|CallOnDrag DragDelta))

(event Custom|CallOnTap
  ;[1 1 1] Tap Component Events
  (Default|CallOnTap)
  (Development|PrintString "Tap"))

(event Custom|CallOnRotate
  (params (RotateDelta :type Float%20%28single-precision%29))
  ;[0 0.3278 0] Rotate Component Events
  (switch Utilities|FlowControl|Switch|SwitchonEnumPinchRotate (Variables|Default|GetPinchRotate)
    (:NewEnumerator0
      (Default|CallOnRotate RotateDelta) ; For rotate 2 fingers
    )))

(event Custom|CallOnSwipe
  (params (SwipeDirection :type Vector%202D%20Structure))
  ;[1 1 1] Swipe Component Events
  (Default|CallOnSwipe SwipeDirection)
  (Development|PrintString "Swipe direction"))

(event EventBeginPlay
  ;[1 1 1] Set GM, tap comp
  (bind _output_get (Variables|/Game/AR_Furniture/Blueprints/TouchComponents/B_TapComponent.B_TapComponent_C|SetGestureManager (Variables|Default|GetTapComponent) self))
  ;[1 1 1] Set GM, drag comp
  (bind _output_get_2 (Variables|/Game/AR_Furniture/Blueprints/TouchComponents/B_DragComponent.B_DragComponent_C|SetGestureManager (Variables|Default|GetDragComponent) _output_get))
  ;[1 1 1] Set GM, swipe comp
  (bind _output_get_3 (Variables|/Game/AR_Furniture/Blueprints/TouchComponents/B_SwipeComponent.B_SwipeComponent_C|SetGestureManager (Variables|Default|GetSwipeComponent) _output_get_2))
  ;[1 1 1] Set GM, pitch comp
  (bind _output_get_4 (Variables|/Game/AR_Furniture/Blueprints/TouchComponents/B_PinchComponent.B_PinchComponent_C|SetGestureManager (Variables|Default|GetPinchComponent) _output_get_3))
  ;[1 1 1] Set GM, rotate comp
  (Variables|/Game/AR_Furniture/Blueprints/TouchComponents/B_RotateComponent.B_RotateComponent_C|SetGestureManager (Variables|Default|GetRotateComponent) _output_get_4))

(event Input|TouchEvents|InputTouch
  (params (Location :type Vector) (FingerIndex :type ETouchIndex%20Enum))
  (bind _tapcomponent (Variables|Default|GetTapComponent))
  (bind _swipecomponent (Variables|Default|GetSwipeComponent))
  (:Pressed
    (Variables|Default|SetID_Finger FingerIndex)
    (Utilities|FlowControl|Sequence
      (:then_0
        (bind _touchposition (CallFunction|GetTouchPosition (Variables|Default|GetID_Finger)))
        (Utilities|FlowControl|Sequence
          (:then_0
            ;[1 1 1] Sign to tap component event
            (Default|Finger1Pressed _tapcomponent _touchposition)
            ;[1 1 1] Sign to tap component event
            (Default|Finger1Pressed (Variables|Default|GetDragComponent) _touchposition)
            ;[1 1 1] Sing to swipe component event
            (Default|Finger1Pressed _swipecomponent _touchposition))
          (:then_1
            (Timeline|Finger1_Timeline Play
              (:Update
                (bind _touchposition_2 (CallFunction|GetTouchPosition (Variables|Default|GetID_Finger)))
                ;[1 1 1] Finger1 Timeline update
                (Default|Finger1Update (Variables|Default|GetDragComponent) _touchposition_2))))))
      (:then_1
        (bind _touchposition_3 (CallFunction|GetTouchPosition (Variables|Default|GetID_Finger)))
        (if (Utilities|Enum|Equal(Enum) "Touch2" (Variables|Default|GetID_Finger))
          (Utilities|FlowControl|Sequence
            (:then_0
              (Timeline|Finger1_Timeline Stop))
            (:then_1
              ;[1 1 1] PitchComponent
              (Default|StartPitch (Variables|Default|GetPinchComponent) _touchposition_3 (stale _touchposition_7))
              ;[1 1 1] Rotate Component
              (Default|StartRotate (Variables|Default|GetRotateComponent) _touchposition_3 (stale _touchposition_7)))
            (:then_2
              (Timeline|TwoFingersUpdate Play
                (:Update
                  (bind _touchposition_4 (CallFunction|GetTouchPosition "Touch1"))
                  (bind _touchposition_5 (CallFunction|GetTouchPosition "Touch2"))
                  ;[1 1 1] Pitch Component
                  (Default|UpdatePitch (Variables|Default|GetPinchComponent) _touchposition_4 _touchposition_5)
                  ;[1 1 1] Rotate Component
                  (Default|UpdateRotate (Variables|Default|GetRotateComponent) _touchposition_4 _touchposition_5)))))))))
  (:Released
    (Variables|Default|SetID_Finger FingerIndex)
    (Utilities|FlowControl|Sequence
      (:then_0
        (bind _touchposition_6 (CallFunction|GetTouchPosition (Variables|Default|GetID_Finger)))
        (Utilities|FlowControl|Sequence
          (:then_0
            (Default|Finger1Released _tapcomponent _touchposition_6)
            (Default|Finger1Released _swipecomponent _touchposition_6))
          (:then_1
            (Timeline|Finger1_Timeline Stop))
          (:then_2
            (Timeline|TwoFingersUpdate Stop))))
      (:then_1
        (bind _touchposition_7 (CallFunction|GetTouchPosition (Variables|Default|GetID_Finger)))
        (Timeline|TwoFingersUpdate Stop)))))

(fn ConstructionScript)

(fn GetTouchPosition
  (params (FingerIndex :type ETouchIndex%20Enum :default "Touch1"))
  (bind _returnvalue (Game|GetPlayerController 0))
  (bind (_locationx _locationy) (Class|PlayerController|GetInputTouchState _returnvalue FingerIndex))
  (return (Math|Vector2D|MakeVector2D _locationx _locationy)))