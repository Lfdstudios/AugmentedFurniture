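; B_DragComponent is a touch component that detects one-finger drag gestures in the AR Furniture project.
; It stores the touch position on press and, on each update, measures how far the finger has moved since then or since the last reported drag.
; When that distance exceeds DragThreshold, it passes the delta (previous minus current) to the GestureManager's drag call and resets the reference position.
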(event Custom|Finger1_Pressed
  (params (TouchPosition :type Vector%202D%20Structure))
  (Variables|Default|SetPreviousPosition TouchPosition))

(event Custom|Finger1_Update
  (params (TouchPos :type Vector%202D%20Structure))
  (bind _output_get (Variables|Default|SetCurrentPosition TouchPos))
  (if (> (Math|Vector2D|Vector2DLength (- (Variables|Default|GetPreviousPosition) (Variables|Default|GetCurrentPosition))) (Variables|Default|GetDragThreshold))
    (Default|CallonDrag (Variables|Default|GetGestureManager) (- (Variables|Default|GetPreviousPosition) (Variables|Default|GetCurrentPosition)))
    (Variables|Default|SetPreviousPosition _output_get)))