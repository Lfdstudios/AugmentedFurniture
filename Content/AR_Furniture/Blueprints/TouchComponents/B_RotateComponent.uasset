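; Touch component for the AR furniture app that turns a two-finger twist gesture into rotation events on the GestureManager.
; StartRotate stores the initial vector between the fingers, and UpdateRotate measures the signed Atan2 angle from it to the current vector.
; Angle changes above RotateThreshold are sent as deltas, while large jumps, such as angle wrap-around, update the stored angle without being sent.
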(event Custom|StartRotate
  (params (Finger1_TouchPos :type Vector%202D%20Structure) (Finger2_TouchPos :type Vector%202D%20Structure))
  (Variables|Default|SetStartDirection (- Finger1_TouchPos Finger2_TouchPos))
  (Variables|Default|SetPreviousAngle 0.0))

(event Custom|UpdateRotate
  (params (Finger1_TouchPos :type Vector%202D%20Structure) (Finger2_TouchPos :type Vector%202D%20Structure))
  (bind _angle (CallFunction|AngleBetweenVectors (- Finger1_TouchPos Finger2_TouchPos) (Variables|Default|GetStartDirection)))
  (if (> (Math|Float|Absolute(Float) (- _angle (Variables|Default|GetPreviousAngle))) (Variables|Default|GetRotateThreshold))
    (if (< (Math|Float|Absolute(Float) (- _angle (Variables|Default|GetPreviousAngle))) 1e+01)
      (Default|CallonRotate (Variables|Default|GetGestureManager) (- _angle (Variables|Default|GetPreviousAngle))))
    (Variables|Default|SetPreviousAngle _angle)))

(fn DotProduct
  (params (FirstVector :type Vector%202D%20Structure) (SecondVector :type Vector%202D%20Structure))
  (bind (_x _y) (Math|Vector2D|BreakVector2D SecondVector))
  (bind (_x_2 _y_2) (Math|Vector2D|BreakVector2D FirstVector))
  (return (+ (* _x_2 _x) (* _y_2 _y))))

(fn AngleBetweenVectors
  (params (FirstVector :type Vector%202D%20Structure) (SecondVector :type Vector%202D%20Structure))
  (bind (_x _y) (Math|Vector2D|BreakVector2D FirstVector))
  (bind (_x_2 _y_2) (Math|Vector2D|BreakVector2D SecondVector))
  (return (- (Class|KismetMathLibrary|DegAtan2 _y _x) (Class|KismetMathLibrary|DegAtan2 _y_2 _x_2))))