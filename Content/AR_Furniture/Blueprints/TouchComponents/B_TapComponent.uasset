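; Touch component for the AR furniture project that detects single-finger taps and double taps and reports them to the GestureManager.
; The first press stores its position and opens a timed window with a Delay.
; A second press close enough within that window fires OnDoubleTap, and any release within it fires OnTap immediately, so taps also fire during double taps.
; An enum switch gates both calls, and GetTouchPosit is an empty stub.
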(event Custom|Finger1_Pressed
  (params (TouchPosition :type Vector%202D%20Structure))
  (if (Variables|Default|GetIsTap)
    (if (< (Math|Vector2D|Vector2DLength (- TouchPosition (Variables|Default|GetStartTouchPosition))) (Variables|Default|GetDoubleTapDistance))
      (switch Utilities|FlowControl|Switch|SwitchonEnumTap (Variables|Default|GetSwitch%20Enum)
        (:NewEnumerator1
          (Default|CallonDoubleTap (Variables|Default|GetGestureManager)))))
    (else
      (Variables|Default|SetStartTouchPosition TouchPosition)
      (Variables|Default|SetIsTap true)
      (Utilities|FlowControl|Delay (Variables|Default|GetDoubleTapDelay))
      (Variables|Default|SetIsTap false))))

(event Custom|Finger1_Released
  (params (TouchPosition :type Vector%202D%20Structure))
  (if (Variables|Default|GetIsTap)
    (switch Utilities|FlowControl|Switch|SwitchonEnumTap (Variables|Default|GetSwitch%20Enum)
      (:NewEnumerator1
        (Default|CallonTap (Variables|Default|GetGestureManager))))))

(fn GetTouchPosit)