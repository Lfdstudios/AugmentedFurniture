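; Placeable AR washbasin actor that can be dragged, rotated or scaled, destroyed by a quick double tap, and has two animated doors.
; BeginPlay and body touches bind GestureManager events, choosing rotate or pinch from the pawn's action enum; UnpressUnbindFatherBP clears them.
; Drag follows camera axes and scale is clamped.
; FlipFlop timelines swing the doors, gated by NoOpen during manipulation, and EndPlay decrements the pawn's spawn count.
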(event OnInputTouchBegin(StaticMesh)
  (params (FingerIndex :type ETouchIndex%20Enum :default "Touch1") (TouchedComponent :type Primitive%20Component%20Object%20Reference))
  (Variables|Default|SetNoOpen false) ; If we touch NO open doors
  (Utilities|FlowControl|Sequence
    (:then_0
      (Variables|Default|SetTap true)
      (EventDispatchers|BindEventtoOnDrag (stale EventBeginPlay _output_get) (delegate Custom|EventDrag))
      (EventDispatchers|BindEventtoOnDoubleTap (Variables|Default|GetGestureManager) (delegate Custom|EventDoubleTap))
      (switch Utilities|FlowControl|Switch|SwitchonEnumMeshes (Variables|/Game/AR_Furniture/Blueprints/B_ARPawn.B_ARPawn_C|GetEnumAction (Variables|Default|GetB_ARPawn)) ; Rotare or Scale ?
        (:NewEnumerator0
          (CallFunction|BindRotate))
        (:NewEnumerator1
          (CallFunction|BindonPinch))))
    (:then_1
      ;[1 1 1] After 0.2 no Destroy evalible
      (Utilities|FlowControl|RetriggerableDelay 0.2)
      (Variables|Default|SetTap false))))

(event OnInputTouchBegin(StaticMesh2)
  (params (FingerIndex :type ETouchIndex%20Enum :default "Touch1") (TouchedComponent :type Primitive%20Component%20Object%20Reference))
  (Variables|Default|SetNoOpen false) ; If we touch NO open doors
  (Utilities|FlowControl|Sequence
    (:then_0
      (Variables|Default|SetTap true)
      (EventDispatchers|BindEventtoOnDrag (stale EventBeginPlay _output_get) (delegate Custom|EventDrag))
      (EventDispatchers|BindEventtoOnDoubleTap (Variables|Default|GetGestureManager) (delegate Custom|EventDoubleTap))
      (switch Utilities|FlowControl|Switch|SwitchonEnumMeshes (Variables|/Game/AR_Furniture/Blueprints/B_ARPawn.B_ARPawn_C|GetEnumAction (Variables|Default|GetB_ARPawn)) ; Rotare or Scale ?
        (:NewEnumerator0
          (CallFunction|BindRotate))
        (:NewEnumerator1
          (CallFunction|BindonPinch))))
    (:then_1
      ;[1 1 1] After 0.2 no Destroy evalible
      (Utilities|FlowControl|RetriggerableDelay 0.2)
      (Variables|Default|SetTap false))))

(event OnInputTouchBegin(StaticMesh3)
  (params (FingerIndex :type ETouchIndex%20Enum :default "Touch1") (TouchedComponent :type Primitive%20Component%20Object%20Reference))
  (if (Variables|Default|GetNoOpen)
    (CallFunction|DoTouch TouchedComponent)))

(event OnInputTouchBegin(StaticMesh4)
  (params (FingerIndex :type ETouchIndex%20Enum :default "Touch1") (TouchedComponent :type Primitive%20Component%20Object%20Reference))
  (if (Variables|Default|GetNoOpen)
    (CallFunction|DoTouch TouchedComponent)))

(event Custom|EventDrag
  (params (DragDelta :type Vector%202D%20Structure))
  (CallFunction|DragMesh (* DragDelta 0.25)))

(event Custom|EventDoubleTap
  (if (Variables|Default|GetTap)
    (Actor|DestroyActor self)
    (Variables|Default|SetTap false)))

(event Custom|OnRotateEventt
  (params (RotateDelta :type Float%20%28single-precision%29))
  ;[1 1 1] Rotate
  (CallFunction|RotateMesh RotateDelta)
  (Variables|Default|SetNoOpen false) ; When rotate cannot open doors
)

(event Custom|OnPinchEvent
  (params (PinchDelta :type Float%20%28single-precision%29))
  ;[1 1 1] Scale
  (CallFunction|ScaleMesh (* PinchDelta 0.01))
  (Variables|Default|SetNoOpen false) ; When scale cannot open doors
)

(event EventBeginPlay
  (|CallParentFunction)
  ;[1 1 1] Set value to the local variable
  (bind _output_get (Variables|Default|SetGestureManager (Variables|/Game/AR_Furniture/Blueprints/B_ARPawn.B_ARPawn_C|GetGestureManager (Variables|Default|GetB_ARPawn))))
  (EventDispatchers|BindEventtoOnDrag _output_get (delegate Custom|EventDrag))
  (EventDispatchers|BindEventtoOnDoubleTap (Variables|Default|GetGestureManager) (delegate Custom|EventDoubleTap))
  (switch Utilities|FlowControl|Switch|SwitchonEnumMeshes (Variables|/Game/AR_Furniture/Blueprints/B_ARPawn.B_ARPawn_C|GetEnumAction (Variables|Default|GetB_ARPawn)) ; Rotare or Scale ?
    (:NewEnumerator0
      (CallFunction|BindRotate))
    (:NewEnumerator1
      (CallFunction|BindonPinch))))

(event Collision|EventActorBeginOverlap
  (params (OtherActor :type Actor%20Object%20Reference))
  (|CallParentFunction OtherActor) ; This node is disabled and will not be called.\nDrag off pins to build functionality.
)

(event EventUnpressUnbindFatherBP
  ;[1 1 1] Unbind all events on detach in ARPawn
  (Development|PrintString "Unpress" true true "(R=0.923461,G=0.000000,B=1.000000,A=1.000000)")
  (EventDispatchers|UnbindallEventsfromOnDrag (Variables|Default|GetGestureManager))
  (EventDispatchers|UnbindallEventsfromOnDoubleTap (Variables|Default|GetGestureManager))
  (CallFunction|UnbindonPinch)
  (CallFunction|UnbindRotate)
  (Variables|Default|SetNoOpen true) ; Now we can open doors
)

(event EventDoTouch
  (params (Component :type Primitive%20Component%20Object%20Reference))
  (if (== Component (Variables|Default|GetStaticMesh3))
    (Utilities|FlowControl|FlipFlop
      (:A
        (bind _newtrack_0 (Timeline|Timeline_0 Play)
          (:Update
            ;[1 1 1] Right Part
            (Transformation|SetRelativeRotation (Variables|Default|GetStaticMesh3) (Math|Rotator|MakeRotator 0.0 0.0 _newtrack_0) false false))))
      (:B
        (Timeline|Timeline_0 Reverse)))
    (elif (== Component (Variables|Default|GetStaticMesh4))
      (Utilities|FlowControl|FlipFlop
        (:A
          (bind _newtrack_0_2 (Timeline|Timeline_1 Play)
            (:Update
              ;[1 1 1] Left Part
              (Transformation|SetRelativeRotation (Variables|Default|GetStaticMesh4) (Math|Rotator|MakeRotator 0.0 0.0 _newtrack_0_2) false false))))
        (:B
          (Timeline|Timeline_1 Reverse))))))

(event EventUnbindRotate
  (EventDispatchers|UnbindallEventsfromOnRotate (Variables|Default|GetGestureManager)))

(event EventBindRotate
  (EventDispatchers|BindEventtoOnRotate (Variables|Default|GetGestureManager) (delegate Custom|OnRotateEventt))
  (CallFunction|UnbindonPinch))

(event EventBindonPinch
  (EventDispatchers|BindEventtoOnPinch (Variables|Default|GetGestureManager) (delegate Custom|OnPinchEvent))
  (CallFunction|UnbindRotate))

(event EventUnbindonPinch
  (EventDispatchers|UnbindallEventsfromOnPinch (Variables|Default|GetGestureManager)))

(event EventEndPlay
  (params (EndPlayReason :type EEndPlayReason%20Enum :default "Destroyed"))
  ;[1 1 1] Decrement count of the actors
  (Math|Integer|DecrementInt (Variables|/Game/AR_Furniture/Blueprints/B_ARPawn.B_ARPawn_C|GetMaxSpawnedActors (Variables|Default|GetB_ARPawn))))

(fn ConstructionScript
  (|CallParentFunction))

(fn DragMesh
  (params (Delta :type Vector%202D%20Structure))
  (bind (_x _y) (Math|Vector2D|BreakVector2D Delta))
  (bind _b_arpawn (Variables|Default|GetB_ARPawn))
  (bind _camera (Variables|/Game/AR_Furniture/Blueprints/B_ARPawn.B_ARPawn_C|GetCamera _b_arpawn))
  (bind _returnvalue (Math|Vector|GetForwardVector _camera))
  (bind _returnvalue_2 (Math|Vector|GetRightVector _camera))
  (Transformation|AddWorldOffset (Variables|Default|GetStaticMesh3Cube) (+ (* (Math|Vector|Normalize (Math|Vector|MakeVector (.x _returnvalue_2) (.y _returnvalue_2) (.z _returnvalue_2))) (* _x -1.0)) (* (Math|Vector|Normalize (Math|Vector|MakeVector (.x _returnvalue) (.y _returnvalue) 0.0)) _y)) false false))

(fn ScaleMesh
  (params (Pinchh :type Float%20%28single-precision%29))
  (bind _staticmesh3cube (Variables|Default|GetStaticMesh3Cube))
  (Transformation|SetWorldScale3D _staticmesh3cube (Math|Vector|ClampVectorSize (+ (* "1.000000,1.000000,1.000000" Pinchh) (Transformation|GetWorldScale _staticmesh3cube)) 1.0 7.0)))

(fn RotateMesh
  (params (RotateDeltaa :type Float%20%28single-precision%29))
  (Transformation|AddWorldRotation (Variables|Default|GetStaticMesh3Cube) (Math|Rotator|MakeRotator 0.0 0.0 RotateDeltaa) false false))