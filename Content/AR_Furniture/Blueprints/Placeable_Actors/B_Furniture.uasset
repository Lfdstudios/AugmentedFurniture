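; Placeable AR furniture actor whose mesh, set from a widget, can be dragged, rotated, scaled or removed by touch.
; BeginPlay and mesh touches bind the pawn's GestureManager events, with the pawn's action enum selecting either twist-to-rotate or pinch-to-scale.
; Drag follows camera axes, scale is clamped, and double-tap destroys only briefly after touching the mesh.
; An unpress event unbinds gestures, and EndPlay decrements the pawn's spawn counter.
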(event OnInputTouchBegin(StaticMesh)
  (params (FingerIndex :type ETouchIndex%20Enum :default "Touch1") (TouchedComponent :type Primitive%20Component%20Object%20Reference))
  (Variables|Default|SetFingerID FingerIndex)
  (Utilities|FlowControl|Sequence
    (:then_0
      (Variables|Default|SetTap true)
      (EventDispatchers|BindEventtoOnDrag (stale EventBeginPlay _output_get) (delegate Custom|OnDragEvent))
      (EventDispatchers|BindEventtoOnDoubleTap (Variables|Default|GetGestureManager) (delegate Custom|Destroy))
      (switch Utilities|FlowControl|Switch|SwitchonEnumMeshes (Variables|/Game/AR_Furniture/Blueprints/B_ARPawn.B_ARPawn_C|GetEnumAction (Variables|Default|GetB_ARPawn)) ; Rotare or Scale ?
        (:NewEnumerator0
          (CallFunction|BindRotate))
        (:NewEnumerator1
          (CallFunction|BindonPinch))))
    (:then_1
      ;[1 1 1] After 0.2 no Destroy evalible
      (Utilities|FlowControl|RetriggerableDelay 0.2)
      (Variables|Default|SetTap false))))

(event Custom|OnDragEvent
  (params (DragDelta :type Vector%202D%20Structure))
  (CallFunction|DragMesh (* DragDelta 0.25)))

(event Custom|Destroy
  (if (Variables|Default|GetTap)
    (Actor|DestroyActor self)
    (Variables|Default|SetTap false)))

(event Custom|OnRotateEvent
  (params (RotateDelta :type Float%20%28single-precision%29))
  ;[1 1 1] Rotate
  (if (Utilities|Enum|Equal(Enum) (Variables|Default|GetFingerID) "Touch2")
    (CallFunction|RotateMesh RotateDelta)))

(event Custom|OnPinchEvent
  (params (PinchDelta :type Float%20%28single-precision%29))
  ;[1 1 1] Scale
  (if (Utilities|Enum|Equal(Enum) (Variables|Default|GetFingerID) "Touch2")
    (CallFunction|ScaleMesh (* PinchDelta 0.01))))

(event EventBeginPlay
  (|CallParentFunction)
  (Components|StaticMesh|SetStaticMesh (Variables|Components|GetStaticMesh) (Variables|Default|GetNewStaticMesh))
  ;[1 1 1] Set value to the local variable
  (bind _output_get (Variables|Default|SetGestureManager (Variables|/Game/AR_Furniture/Blueprints/B_ARPawn.B_ARPawn_C|GetGestureManager (Variables|Default|GetB_ARPawn))))
  (EventDispatchers|BindEventtoOnDrag _output_get (delegate Custom|OnDragEvent))
  (EventDispatchers|BindEventtoOnDoubleTap (Variables|Default|GetGestureManager) (delegate Custom|Destroy))
  (switch Utilities|FlowControl|Switch|SwitchonEnumMeshes (Variables|/Game/AR_Furniture/Blueprints/B_ARPawn.B_ARPawn_C|GetEnumAction (Variables|Default|GetB_ARPawn)) ; Rotare or Scale ?
    (:NewEnumerator0
      (CallFunction|BindRotate))
    (:NewEnumerator1
      (CallFunction|BindonPinch))))

(event Collision|EventActorBeginOverlap
  (params (OtherActor :type Actor%20Object%20Reference))
  (|CallParentFunction OtherActor) ; This node is disabled and will not be called.\nDrag off pins to build functionality.
)

(event EventTick
  (params (DeltaSeconds :type Float%20%28single-precision%29))
  (|CallParentFunction DeltaSeconds))

(event EventUnpressUnbindFatherBP
  ;[1 1 1] Unbind all events on detach in ARPawn
  (Development|PrintString "Unpress" true true "(R=0.923461,G=0.000000,B=1.000000,A=1.000000)")
  (EventDispatchers|UnbindallEventsfromOnDrag (Variables|Default|GetGestureManager))
  (EventDispatchers|UnbindallEventsfromOnDoubleTap (Variables|Default|GetGestureManager))
  (CallFunction|UnbindonPinch)
  (CallFunction|UnbindRotate))

(event EventUnbindRotate
  (EventDispatchers|UnbindallEventsfromOnRotate (Variables|Default|GetGestureManager)))

(event EventBindRotate
  (EventDispatchers|BindEventtoOnRotate (Variables|Default|GetGestureManager) (delegate Custom|OnRotateEvent))
  (CallFunction|UnbindonPinch))

(event EventBindonPinch
  (EventDispatchers|BindEventtoOnPinch (Variables|Default|GetGestureManager) (delegate Custom|OnPinchEvent))
  (CallFunction|UnbindRotate))

(event EventUnbindonPinch
  (EventDispatchers|UnbindallEventsfromOnPinch (Variables|Default|GetGestureManager)))

(event EventEndPlay
  (params (EndPlayReason :type EEndPlayReason%20Enum :default "Destroyed"))
  ;[1 1 1] Decrement count of the actors
  (Math|Integer|DecrementInt (Variables|/Game/AR_Furniture/Blueprints/B_ARPawn.B_ARPawn_C|GetMaxSpawnedActors (Variables|Default|GetB_ARPawn))))

(fn ConstructionScript
  (|CallParentFunction))

(fn DragMesh
  (params (Delta :type Vector%202D%20Structure))
  (bind (_x _y) (Math|Vector2D|BreakVector2D Delta))
  (bind _b_arpawn (Variables|Default|GetB_ARPawn))
  (bind _camera (Variables|/Game/AR_Furniture/Blueprints/B_ARPawn.B_ARPawn_C|GetCamera _b_arpawn))
  (bind _returnvalue (Math|Vector|GetForwardVector _camera))
  (bind _returnvalue_2 (Math|Vector|GetRightVector _camera))
  (Transformation|AddWorldOffset (Variables|Components|GetStaticMesh) (+ (* (Math|Vector|Normalize (Math|Vector|MakeVector (.x _returnvalue_2) (.y _returnvalue_2) (.z _returnvalue_2))) (* _x -1.0)) (* (Math|Vector|Normalize (Math|Vector|MakeVector (.x _returnvalue) (.y _returnvalue) 0.0)) _y)) false false))

(fn ScaleMesh
  (params (Pinchh :type Float%20%28single-precision%29))
  (bind _staticmesh (Variables|Components|GetStaticMesh))
  (Transformation|SetWorldScale3D _staticmesh (Math|Vector|ClampVectorSize (+ (* "1.000000,1.000000,1.000000" Pinchh) (Transformation|GetWorldScale _staticmesh)) 1.0 7.0)))

(fn RotateMesh
  (params (RotateDeltaa :type Float%20%28single-precision%29))
  (Transformation|AddWorldRotation (Variables|Components|GetStaticMesh) (Math|Rotator|MakeRotator 0.0 0.0 RotateDeltaa) false false))